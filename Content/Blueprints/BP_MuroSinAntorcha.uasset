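; BP_MuroSinAntorcha is a wall that keeps the player from passing until they have the torch.
; On Box overlap it casts to BP_MainCharacter and destroys itself if HasTorch is true.
; Otherwise, a DoOnce plays a thinking sound, calls EventDialog and briefly shows a Dialog_UI widget.
; A parallel Sequence branch resets the DoOnce after a delay, throttling repeat hints.
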(event OnComponentBeginOverlap(Box)
  (params (OverlappedComponent :type Primitive%20Component%20Object%20Reference) (OtherActor :type Actor%20Object%20Reference) (OtherComp :type Primitive%20Component%20Object%20Reference) (OtherBodyIndex :type Integer) (bFromSweep :type Boolean) (SweepResult :type Hit%20Result%20Structure%20%28by%20ref%29))
  ;[1 1 1] Revisa si el jugador ya tiene la antorcha y no lo deja pasar hasta que la tenga
  (bind _asbp_main_character (Utilities|Casting|CastToBP_MainCharacter OtherActor))
  (if (Variables|/Game/Blueprints/Characters/Player/BP_MainCharacter.BP_MainCharacter_C|GethasTorch _asbp_main_character)
    (Actor|DestroyActor)
    (else
      (Utilities|FlowControl|Sequence
        (:then_0
          (Utilities|FlowControl|DoOnce false :!label _label
            (:Completed
              (Audio|PlaySoundatLocation "/Game/Audio/sfx/Player/ThinkingSound.ThinkingSound" "0, 0, 0" "0, 0, 0" 1.0 1.0 0.0 0 0 0 0)
              (CallFunction|EventDialog)
              (bind _returnvalue (UserInterface|CreateWidget "/Game/Maps/Victor/Dialog_UI.Dialog_UI_C"))
              (UserInterface|Viewport|AddtoViewport _returnvalue 0)
              (Utilities|FlowControl|Delay 3.0)
              (Widget|RemovefromParent _returnvalue))))
        (:then_1
          (Utilities|FlowControl|Delay 5.0)
          (goto _label Reset))))))

(event EventBeginPlay)

(event Collision|EventActorBeginOverlap
  (params (OtherActor :type Actor%20Object%20Reference)))

(event EventTick
  (params (DeltaSeconds :type Float%20%28single-precision%29)))

(fn ConstructionScript)